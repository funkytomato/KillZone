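; Interaction component that lets the player interact with objects in the world through a line trace.
; It caches the player character on BeginPlay, and InteractEvent traces on Visibility from the first-person camera along the root component's forward vector, not the camera's.
; A hit prints the component name and sends an interaction interface message to the hit actor, adding Pickup when ObjectPickedUp is set.
; Debug trace drawing is enabled.
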(event `self.ReceiveBeginPlay`
  ;[1 1 1] BeginPlay - Get Player Character Reference
  (bind _asplayer_character_bp (cast `/Game/MyContent/Blueprints/Characters/MyPlayerCharacter_BP` (`GameplayStatics.GetPlayerCharacter` 0)))
  (set `self.PlayerCharacter` _asplayer_character_bp))

(event `InteractEvent`
  (bind _playercharacter (`self.PlayerCharacter`))
  (bind _returnvalue (`SceneComponent.K2_GetComponentLocation` (`/Game/MyContent/Blueprints/Characters/MyPlayerCharacter_BP.FirstPersonCamera` _playercharacter)))
  ;[1 1 1] Interact with object
  (bind (_outhit _returnvalue_2) (`KismetSystemLibrary.LineTraceSingle` :`Start` _returnvalue :`End` (+ _returnvalue (* (`KismetMathLibrary.GetForwardVector` (`SceneComponent.K2_GetComponentRotation` (`Actor.RootComponent` _playercharacter))) 8000.0)) :`TraceChannel` "TraceTypeQuery1" :`DrawDebugType` "ForDuration" :`DrawTime` 1.0))
  (if _returnvalue_2
    (bind (_bblockinghit _binitialoverlap _time _distance _location _impactpoint _normal _impactnormal _physmat _hitactor _hitcomponent) (`GameplayStatics.BreakHitResult` _outhit))
    (`KismetSystemLibrary.PrintString` (`KismetSystemLibrary.GetDisplayName` _hitcomponent))
    (if (`self.ObjectPickedUp`)
      (message `/Game/BallisticsVFX/FirstPersonBPExamples/BPI_Interaction.BPI_Interaction` _hitactor (`self.PlayerCharacter`) _hitcomponent (`self.Pickup`))
      (else
        (message `/Game/BallisticsVFX/FirstPersonBPExamples/BPI_Interaction.BPI_Interaction` _hitactor (`self.PlayerCharacter`) _hitcomponent null)))))