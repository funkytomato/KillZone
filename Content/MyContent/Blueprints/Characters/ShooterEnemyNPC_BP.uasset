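; Armed enemy NPC that shoots with a child-actor gun set up as rifle, pistol or HP rifle.
; Projectile hits turn it toward the player and pick hit or death montages by weapon type and bone, which damage events play before death destroys it.
; Threats and cover events switch behavior trees between shoot-from-cover and main shooter AI.
; Trace-based cover helpers can plane-constrain movement and crouch, though height and side checks end in empty branches.
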(event `self.WeaponReload`
  (`parent.WeaponReload`)
  (`/Game/MyContent/Blueprints/Weapons/EnemyBFXGun_BP.Reload` (`self.EquippedGun`)))

(event `StartShooting`
  (`/Game/MyContent/Blueprints/Weapons/EnemyBFXGun_BP.TriggerPressedEvent` (`self.EquippedGun`))
  (set `self.IsShooting?` true))

(event `StopShooting`
  (`/Game/MyContent/Blueprints/Weapons/EnemyBFXGun_BP.TriggerReleasedEvent` (`self.EquippedGun`))
  (set `self.IsShooting?` false))

(event `EnterCover`
  (set `self.Ironsight` true)
  (set `self.IsInCover?` true)
  (`self.StartCrouch`)
  (`AIController.RunBehaviorTree` (`AIBlueprintHelperLibrary.GetAIController` self) "/Game/MyContent/AI/EnemyShootFromCover_BT.EnemyShootFromCover_BT"))

(event `LeaveCover`
  (set `self.IsInCover?` false)
  (`self.StopCrouching`)
  (`AIController.RunBehaviorTree` (`AIBlueprintHelperLibrary.GetAIController` self) "/Game/MyContent/ShooterSimplifiedAI/Blueprints/AI/BehaviorTree/BT_MainShooter_AI.BT_MainShooter_AI"))

(event `self.ReceiveHit`
  (params (MyComp :type "PrimitiveComponent Object Reference") (Other :type "Actor Object Reference") (OtherComp :type "PrimitiveComponent Object Reference") (bSelfMoved :type Boolean) (HitLocation :type "Vector Structure") (HitNormal :type "Vector Structure") (NormalImpulse :type "Vector Structure") (Hit :type "HitResult Structure (by ref)"))
  (`parent.ReceiveHit` MyComp Other OtherComp bSelfMoved HitLocation HitNormal NormalImpulse Hit)
  (cast `/Game/MyContent/BallisticsVFX/FXSpawnerBlueprints/Projectiles/CubitUniProjectile` Other)
  (`self.RotateToAggressor`)
  (`|ExecutionSequence`
    (:`then_0`
      (`self.SelectHitAnimation` (`.HitBoneName` (`GameplayStatics.BreakHitResult` Hit))))
    (:`then_1`
      (if (`/Game/MyContent/Blueprints/Health/Health_CBP.IsDead?` (`self.Health_CBP`))
        (`self.SelectDeathAnimation`)))))

(event `PlayHitAnimation`
  (`CharacterMovementComponent.DisableMovement` (`self.CharacterMovement`) :!label _label)
  (bind _returnvalue (`AnimInstance.Montage_Play` (`self.AnimInstanceRef`) (`self.DamageMontage`) 1.0 "MontageLength" 0.0 true))
  (`KismetSystemLibrary.Delay` _returnvalue)
  (if (not (`/Game/MyContent/Blueprints/Health/Health_CBP.IsDead?` (`self.Health_CBP`)))
    (`CharacterMovementComponent.SetMovementMode` (`self.CharacterMovement`) "MOVE_Walking" 0)
    (`/Engine/EditorBlueprintResources/StandardMacros.DoOnce` false :!via `Reset`
      (:`Completed`
        (goto _label)))))

(event `PlayDeathAnimation`
  (`/Engine/EditorBlueprintResources/StandardMacros.DoOnce` false
    (:`Completed`
      (`CharacterMovementComponent.DisableMovement` (`self.CharacterMovement`))
      (bind _returnvalue (`AnimInstance.Montage_Play` (`self.AnimInstanceRef`) (`self.DamageMontage`) 1.0 "MontageLength" 0.0 true))
      (`KismetSystemLibrary.Delay` (+ _returnvalue 0.5))
      (`self.OnDeath`)
      (`KismetSystemLibrary.Delay` 10.0)
      (`self.K2_DestroyActor`))))

(event `self.ReceiveAnyDamage`
  (params (Damage :type "Float (single-precision)") (DamageType :type "DamageType Object Reference") (InstigatedBy :type "Controller Object Reference") (DamageCauser :type "Actor Object Reference"))
  (`parent.ReceiveAnyDamage` Damage DamageType InstigatedBy DamageCauser)
  (if (`/Game/MyContent/Blueprints/Health/Health_CBP.IsDead?` (`self.Health_CBP`))
    (`self.SelectDeathAnimation`)
    (`self.PlayDeathAnimation`)
    (else
      (`self.PlayHitAnimation`))))

(event `RotateToAggressor`
  (if (not (`/Game/MyContent/Blueprints/Health/Health_CBP.IsDead?` (`self.Health_CBP`)))
    (`self.K2_SetActorRotation` (`KismetMathLibrary.FindLookAtRotation` (`self.K2_GetActorLocation`) (`self.K2_GetActorLocation` (`GameplayStatics.GetPlayerCharacter` 0))))))

(event `StartCrouch`
  (`self.Crouch`)
  (set `self.IsCrouching?` true)
  (bind _asenemy_npc_abp1 (cast `/Game/MyContent/Blueprints/Characters/EnemyNPC_ABP1` (`self.AnimInstanceRef`)))
  (set `/Game/MyContent/Blueprints/Characters/EnemyNPC_ABP1.IsCrouching?` true _asenemy_npc_abp1))

(event `StopCrouching`
  (`self.UnCrouch`)
  (set `self.IsCrouching?` false)
  (bind _asenemy_npc_abp1 (cast `/Game/MyContent/Blueprints/Characters/EnemyNPC_ABP1` (`self.AnimInstanceRef`)))
  (set `/Game/MyContent/Blueprints/Characters/EnemyNPC_ABP1.IsCrouching?` false _asenemy_npc_abp1))

(event `StartProne`
  (set `self.IsProne?` true))

(event `StopProne`
  (set `self.IsProne?` false))

(event `self.ReceiveBeginPlay`
  ;[1 1 1] BeginPlay - Bind to Dead Message
  (`parent.ReceiveBeginPlay`)
  (add `/Game/MyContent/Blueprints/Health/Health_CBP.IsDead` (`self.Health_CBP`) (delegate `Die`)))

(event `Die`
  ;[1 1 1] BeginPlay - Bind to Dead Message
  (bind _asenemy_npc_abp1 (cast `/Game/MyContent/Blueprints/Characters/EnemyNPC_ABP1` (`self.AnimInstanceRef`)))
  (set `/Game/MyContent/Blueprints/Characters/EnemyNPC_ABP1.IsDead?` true _asenemy_npc_abp1))

(event `self.Threatened`
  (params (ThreatOrigin :type "Vector Structure"))
  (bind _returnvalue (`AIBlueprintHelperLibrary.GetAIController` self))
  (`parent.Threatened` ThreatOrigin)
  (`AIController.RunBehaviorTree` _returnvalue "/Game/MyContent/AI/EnemyShootFromCover_BT.EnemyShootFromCover_BT")
  (`AIController.K2_SetFocalPoint` _returnvalue ThreatOrigin))

(fn `CheckForCover`
  (if (`self.IsInCover?`)
    (`self.StopCover`)
    (else
      (`self.WallTrace`))))

(fn `CoverTrace`
  (locals (RightHit :type Boolean :default false) (LeftHit :type Boolean :default false))
  (bind _returnvalue (`MovementComponent.GetPlaneConstraintNormal` (`self.CharacterMovement`)))
  (bind _returnvalue_2 (* (`MovementComponent.GetPlaneConstraintNormal` (`self.CharacterMovement`)) -1.0))
  (bind _returnvalue_3 (* (`KismetMathLibrary.GetRightVector` (`KismetMathLibrary.MakeRotFromX` _returnvalue)) 45.0))
  (bind _returnvalue_4 (* (`KismetMathLibrary.GetRightVector` (`KismetMathLibrary.MakeRotFromX` _returnvalue_2)) 45.0))
  (`|ExecutionSequence`
    (:`then_0`
      (bind (_outhit _returnvalue_5) (`KismetSystemLibrary.LineTraceSingle` (+ (`self.K2_GetActorLocation`) _returnvalue_4) (+ _returnvalue_4 (* _returnvalue_2 200.0)) "TraceTypeQuery3"))
      (set `local.RightHit` _returnvalue_5))
    (:`then_1`
      (bind (_outhit_2 _returnvalue_6) (`KismetSystemLibrary.LineTraceSingle` (+ (`self.K2_GetActorLocation`) _returnvalue_3) (+ _returnvalue_3 (* (* _returnvalue -1.0) 200.0)) "TraceTypeQuery3"))
      (set `local.LeftHit` _returnvalue_6))
    (:`then_2`
      (if (and (`local.RightHit`) (`local.LeftHit`))
        _))))

(fn `HeightTrace`
  (bind (_returnvalue_x _returnvalue_y _returnvalue_z) (`KismetMathLibrary.BreakVector` (`SceneComponent.GetSocketLocation` (`self.Mesh`) "pelvisSocket")))
  (bind _returnvalue (+ (`self.K2_GetActorLocation`) (0.0 0.0 500.0) (* (`self.GetActorForwardVector`) 75.0)))
  (bind (_outhit _returnvalue_2) (`KismetSystemLibrary.SphereTraceSingle` :`Start` _returnvalue :`End` (- _returnvalue (0.0 0.0 500.0)) :`Radius` 10.0 :`TraceChannel` "TraceTypeQuery1" :`DrawDebugType` "ForOneFrame"))
  (if _returnvalue_2
    (set `self.WallHeight` (`.Location` (`GameplayStatics.BreakHitResult` _outhit)))
    (if (`KismetMathLibrary.InRange_FloatFloat` (- _returnvalue_z (.z (`.Location` (`GameplayStatics.BreakHitResult` _outhit)))) -50.0 0.0)
      _)))

(fn `On Dead`
  (`parent.On Dead`)
  ;[1 1 1] Stop Firing Gun
  (`/Game/MyContent/Blueprints/Weapons/EnemyBFXGun_BP.TriggerReleasedEvent` (`self.EquippedGun`)))

(fn `Select Hip Death Animation`
  (set `self.DamageMontage` (select `int` (`KismetMathLibrary.RandomIntegerInRange` 0 2) :`0` "/Game/MyContent/Animations/ShooterAI/RifleHip_Death_1_Montage.RifleHip_Death_1_Montage" :`1` "/Game/MyContent/Animations/ShooterAI/RifleHip_Death_2_Montage.RifleHip_Death_2_Montage" :`2` "/Game/MyContent/Animations/ShooterAI/RifleHip_Death_3_Montage.RifleHip_Death_3_Montage" :!type "AnimMontage Object Reference")))

(fn `SelectDeathAnimation`
  (switch `/Game/MyContent/ShooterSimplifiedAI/Blueprints/AI/E_AI_WeaponType` (`self.AIWeaponType`)
    (:`NewEnumerator0`
      (`self.SelectIronsightDeathAnimation`))
    (:`NewEnumerator1`
      (`self.SelectPistolDeathAnimation`))
    (:`NewEnumerator2`
      (`self.Select Hip Death Animation`))))

(fn `SelectHipHitAnimation`
  (params (Selection :type Name))
  (switch `name` Selection
    (:`Default`
      (set `self.DamageMontage` "/Game/MyContent/Animations/ShooterAI/RifleHip_Hit_React_3_Montage.RifleHip_Hit_React_3_Montage"))
    (:`Upperarm_l`
      (set `self.DamageMontage` "/Game/MyContent/Animations/ShooterAI/RifleHip_Hit_React_1_Montage.RifleHip_Hit_React_1_Montage"))
    (:`Upperarm_r`
      (set `self.DamageMontage` "/Game/MyContent/Animations/ShooterAI/RifleHip_Hit_React_2_Montage.RifleHip_Hit_React_2_Montage"))
    (:`Thigh_l`
      (set `self.DamageMontage` "/Game/MyContent/Animations/ShooterAI/RifleHip_Hit_React_3_Montage.RifleHip_Hit_React_3_Montage"))
    (:`Thigh_r`
      (set `self.DamageMontage` "/Game/MyContent/Animations/ShooterAI/RifleHip_Hit_React_4_Montage.RifleHip_Hit_React_4_Montage"))
    (:`Head`
      (set `self.DamageMontage` "/Game/MyContent/Animations/ShooterAI/RifleHip_Hit_React_3_Montage.RifleHip_Hit_React_3_Montage"))))

(fn `SelectHitAnimation`
  (params (InputPin :type Name))
  (switch `/Game/MyContent/ShooterSimplifiedAI/Blueprints/AI/E_AI_WeaponType` (`self.AIWeaponType`)
    (:`NewEnumerator0`
      (`self.SelectIronsightHitAnimation` InputPin))
    (:`NewEnumerator1`
      (`self.SelectPistolHitAnimation` InputPin))
    (:`NewEnumerator2`
      (`self.SelectHipHitAnimation` InputPin))))

(fn `SelectIronsightDeathAnimation`
  (set `self.DamageMontage` (select `int` (`KismetMathLibrary.RandomIntegerInRange` 0 2) :`0` "/Game/MyContent/Animations/Rifle/Rifle_Death_L_Montage.Rifle_Death_L_Montage" :`1` "/Game/MyContent/Animations/Rifle/Rifle_Death_R_Montage.Rifle_Death_R_Montage" :`2` "/Game/MyContent/Animations/Rifle/Rifle_Death_3_Montage.Rifle_Death_3_Montage" :!type "AnimMontage Object Reference")))

(fn `SelectIronsightHitAnimation`
  (params (Selection :type Name))
  (switch `name` Selection
    (:`Default`
      (set `self.DamageMontage` "/Game/MyContent/Animations/Rifle/Rifle_Hit_C_1_Montage.Rifle_Hit_C_1_Montage"))
    (:`Upperarm_l`
      (set `self.DamageMontage` "/Game/MyContent/Animations/Rifle/Rifle_Hit_L_1_Montage.Rifle_Hit_L_1_Montage"))
    (:`Upperarm_r`
      (set `self.DamageMontage` "/Game/MyContent/Animations/Rifle/Rifle_Hit_R_1_Montage.Rifle_Hit_R_1_Montage"))
    (:`Thigh_l`
      (set `self.DamageMontage` "/Game/MyContent/Animations/Rifle/Rifle_Hit_L_2_Montage.Rifle_Hit_L_2_Montage"))
    (:`Thigh_r`
      (set `self.DamageMontage` "/Game/MyContent/Animations/Rifle/Rifle_Hit_C_1_Montage.Rifle_Hit_C_1_Montage"))
    (:`Head`
      (set `self.DamageMontage` "/Game/MyContent/Animations/Rifle/Rifle_Hit_C_1_Montage.Rifle_Hit_C_1_Montage"))))

(fn `SelectPistolDeathAnimation`
  (set `self.DamageMontage` (select `int` (`KismetMathLibrary.RandomIntegerInRange` 0 1) :`0` "/Game/MyContent/Animations/Pistol/Pistol_Death_L_Montage.Pistol_Death_L_Montage" :`1` "/Game/MyContent/Animations/Pistol/Pistol_Death_L_Montage.Pistol_Death_L_Montage" :!type "AnimMontage Object Reference")))

(fn `SelectPistolHitAnimation`
  (params (Selection :type Name))
  (switch `name` Selection
    (:`Default`
      (set `self.DamageMontage` "/Game/MyContent/Animations/Pistol/Pistol_Hit_C_1_Montage.Pistol_Hit_C_1_Montage"))
    (:`Upperarm_l`
      (set `self.DamageMontage` "/Game/MyContent/Animations/Pistol/Pistol_Hit_L_1_Montage.Pistol_Hit_L_1_Montage"))
    (:`Upperarm_r`
      (set `self.DamageMontage` "/Game/MyContent/Animations/Pistol/Pistol_Hit_R_2_Montage.Pistol_Hit_R_2_Montage"))
    (:`Thigh_l`
      (set `self.DamageMontage` "/Game/MyContent/Animations/Pistol/Pistol_Hit_L_2_Montage.Pistol_Hit_L_2_Montage"))
    (:`Thigh_r`
      (set `self.DamageMontage` "/Game/MyContent/Animations/Pistol/Pistol_Hit_C_1_Montage.Pistol_Hit_C_1_Montage"))
    (:`Head`
      (set `self.DamageMontage` "/Game/MyContent/Animations/Pistol/Pistol_Hit_C_1_Montage.Pistol_Hit_C_1_Montage"))))

(fn `StartCover`
  (params (PlaneNormal :type "Vector Structure"))
  (bind _charactermovement (`self.CharacterMovement`))
  (`MovementComponent.SetPlaneConstraintEnabled` _charactermovement true)
  (`MovementComponent.SetPlaneConstraintNormal` _charactermovement PlaneNormal)
  (set `self.bUseControllerRotationYaw` false)
  (set `self.IsInCover?` true)
  (`self.Crouch`))

(fn `StopCover`
  (`MovementComponent.SetPlaneConstraintEnabled` (`self.CharacterMovement`) false)
  (set `self.bUseControllerRotationYaw` true)
  (set `self.IsInCover?` false)
  (`self.UnCrouch`))

(fn `UserConstructionScript`
  (`parent.UserConstructionScript`)
  (bind _asenemy_bfxgun_bp (cast `/Game/MyContent/Blueprints/Weapons/EnemyBFXGun_BP` (`ChildActorComponent.ChildActor` (`self.Gun`))))
  (set `self.EquippedGun` _asenemy_bfxgun_bp)
  (`SceneComponent.K2_AttachToComponent` (`self.Gun`) (`self.Mesh`) "weapon_rSocket" "SnapToTarget" "SnapToTarget" "SnapToTarget" true)
  (`self.SetOwner` (`self.EquippedGun`) self)
  (set `/Game/MyContent/Blueprints/Weapons/EnemyBFXGun_BP.GunAudioToggle` false (`self.EquippedGun`)))

(fn `WallTrace`
  (bind _returnvalue (`self.K2_GetActorLocation`))
  (bind (_outhit _returnvalue_2) (`KismetSystemLibrary.LineTraceSingle` :`Start` _returnvalue :`End` (+ _returnvalue (* (`self.GetActorForwardVector`) 150.0)) :`TraceChannel` "TraceTypeQuery3" :`DrawDebugType` "ForDuration"))
  (if _returnvalue_2
    (`self.StartCover` (`.Normal` (`GameplayStatics.BreakHitResult` _outhit)))
    (else
      (`self.StopCover`))))

(fn `Weapon Setup`
  (bind _equippedgun (`self.EquippedGun`))
  (`parent.Weapon Setup`)
  ;[1 1 1] Do not show gun parts
  (`/Engine/EditorBlueprintResources/StandardMacros.IsValid` _equippedgun
    (:`Is Valid`
      (`/Game/MyContent/Blueprints/Weapons/EnemyBFXGun_BP.ThirdPersonGunVisibility` _equippedgun)
      ;[1 1 1] Load Appropriate Gun Properties (including mesh)
      (switch `/Game/MyContent/ShooterSimplifiedAI/Blueprints/AI/E_AI_WeaponType` (`self.AIWeaponType`)
        (:`NewEnumerator0`
          (bind _asenemy_bfxgun_bp (cast `/Game/MyContent/Blueprints/Weapons/EnemyBFXGun_BP` (`ChildActorComponent.ChildActor` (`self.Gun`))))
          (`/Game/MyContent/Blueprints/Weapons/EnemyBFXGun_BP.InitialiseWithRifle` _asenemy_bfxgun_bp))
        (:`NewEnumerator1`
          (bind _asenemy_bfxgun_bp_2 (cast `/Game/MyContent/Blueprints/Weapons/EnemyBFXGun_BP` (`ChildActorComponent.ChildActor` (`self.Gun`))))
          (`/Game/MyContent/Blueprints/Weapons/EnemyBFXGun_BP.InitialiseWithPistol` _asenemy_bfxgun_bp_2))
        (:`NewEnumerator2`
          (bind _asenemy_bfxgun_bp_3 (cast `/Game/MyContent/Blueprints/Weapons/EnemyBFXGun_BP` (`ChildActorComponent.ChildActor` (`self.Gun`))))
          (`/Game/MyContent/Blueprints/Weapons/EnemyBFXGun_BP.InitialiseWithHPRifle` _asenemy_bfxgun_bp_3))))))