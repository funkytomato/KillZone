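; EncounterSpace is an area actor that spreads a target call-out among the shooter enemies inside it.
; Its CallOutTarget event receives a location, finds every ShooterEnemyNPC_BP in the level and keeps those overlapping the space.
; For each, where a valid blackboard is found, it writes TargetLocation and sets CanSeePlayer true, acting as shared detection within the encounter.
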(event `CallOutTarget`
  (params (TargetLocation :type "Vector Structure"))
  (bind _returnvalue (`AIBlueprintHelperLibrary.GetBlackboard` null))
  (set `self.TargetLocation` TargetLocation)
  (bind _outactors (`GameplayStatics.GetAllActorsOfClass` "/Game/MyContent/Blueprints/Characters/ShooterEnemyNPC_BP.ShooterEnemyNPC_BP_C"))
  (for _array_element _outactors
    (if (`self.IsOverlappingActor` _array_element)
      (`/Engine/EditorBlueprintResources/StandardMacros.IsValid` _returnvalue
        (:`Is Valid`
          (`BlackboardComponent.SetValueAsVector` _returnvalue "TargetLocation" (`self.TargetLocation`))
          (`BlackboardComponent.SetValueAsBool` _returnvalue "CanSeePlayer" true))))))

(fn `UserConstructionScript`)